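; Player tank Blueprint that, in this graph, handles only orbit-camera aiming and zoom from input axes.
; Azimuth input yaws a gimbal component, while elevation input pitches the spring arm, gated by its target rotation to keep pitch within set limits.
; Zoom slides the camera along its local X axis, scaled by delta time and without limits, whereas both rotation inputs apply raw axis values.
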(event `InputAxis|AimElevation`
  (params (AxisValue :type "Float (single-precision)"))
  (bind (_returnvalue_roll _returnvalue_pitch) (`KismetMathLibrary.BreakRotator` (`SpringArmComponent.GetTargetRotation` (`self.SpringArm`))))
  ;[1 1 1] Camera input binding
  (if (or (and (>= _returnvalue_pitch -70.0) (< AxisValue 0.0)) (and (<= _returnvalue_pitch 5.0) (> AxisValue 0.0)))
    (`SceneComponent.K2_AddLocalRotation` (`self.SpringArm`) (`KismetMathLibrary.MakeRotator` 0.0 AxisValue) false false)))

(event `InputAxis|AimAzimuth`
  (params (AxisValue :type "Float (single-precision)"))
  ;[1 1 1] Camera input binding
  (`SceneComponent.K2_AddLocalRotation` (`self.Azimuth Gimb`) (`KismetMathLibrary.MakeRotator` 0.0 0.0 AxisValue) false false))

(event `InputAxis|AimZoom`
  (params (AxisValue :type "Float (single-precision)"))
  ;[1 1 1] Camera zoom input
  (`SceneComponent.K2_AddLocalOffset` (`self.Camera`) (`KismetMathLibrary.MakeVector` (* AxisValue (`GameplayStatics.GetWorldDeltaSeconds`) 10000.0)) false false))

(fn `UserConstructionScript`)